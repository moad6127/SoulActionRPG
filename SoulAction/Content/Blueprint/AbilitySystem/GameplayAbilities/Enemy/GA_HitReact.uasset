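; GA_HitReact is an enemy gameplay ability that plays a hit reaction montage on the avatar.
; On activation it applies GE_HitReact to the owner and stores the effect handle.
; It fetches the montage through CombatInterface on the avatar, caching the interface and skipping that lookup while it stays valid.
; When the montage completes, blends out, is interrupted or is cancelled, it removes the effect and ends the ability.
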(event `self.K2_ActivateAbility`
  (bind _returnvalue (`self.BP_ApplyGameplayEffectToOwner` "/Game/Blueprint/AbilitySystem/GameplayEffects/GE_HitReact.GE_HitReact_C"))
  (set `self.ActiveGE_HitRecat` _returnvalue)
  (if (not (`KismetSystemLibrary.IsValidInterface` (`self.CombatInterface`)))
    (bind _ascombat_interface (cast `CombatInterface` (`self.GetAvatarActorFromActorInfo`)))
    (bind _output_get (set `self.CombatInterface` _ascombat_interface))
    (bind _returnvalue_2 (`CombatInterface.GetHitReactMontage` _output_get)))
  (`AbilityTask_PlayMontageAndWait.CreatePlayMontageAndWaitProxy` "None" _returnvalue_2
    (:`OnCompleted`
      _)
    (:`OnBlendOut`
      _)
    (:`OnInterrupted`
      _)
    (:`OnCancelled`
      _))
  (`self.BP_RemoveGameplayEffectFromOwnerWithHandle` (`self.ActiveGE_HitRecat`))
  (`self.K2_EndAbility`))