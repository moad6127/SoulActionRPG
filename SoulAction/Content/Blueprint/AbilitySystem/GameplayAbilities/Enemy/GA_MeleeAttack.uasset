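; Enemy melee attack gameplay ability that turns the avatar toward its combat target and plays a spear attack montage.
; While the montage plays, it waits for the melee montage gameplay event, then finds live players within a small radius of the combat socket, ignoring itself.
; It damages each one and ends the ability, which also ends if the montage completes, is interrupted or is cancelled.
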(event `self.K2_ActivateAbility`
  (bind _returnvalue (`self.GetAvatarActorFromActorInfo`))
  (bind _returnvalue_2 (`self.GetAvatarActorFromActorInfo`))
  (bind _returnvalue_3 (message `EnemyInterface.GetCombatTarget` _returnvalue_2))
  (bind _ascombat_interface (cast `CombatInterface` _returnvalue_2))
  (`CombatInterface.UpdateFacingTarget` _ascombat_interface (`Actor.K2_GetActorLocation` _returnvalue_3))
  (`AbilityTask_PlayMontageAndWait.CreatePlayMontageAndWaitProxy` "None" "/Game/FabContent/Assets/Enemies/Goblin/Animations/Spear/AM_Attack_Spear.AM_Attack_Spear"
    (:`then`
      (`AbilityTask_WaitGameplayEvent.WaitGameplayEvent` (struct :`TagName` "Event.Montage.Attack.Melee") null
        (:`EventReceived`
          (bind _returnvalue_4 (message `CombatInterface.GetCombatSocketLocation` _returnvalue))
          (bind _outoverlappingactors (`SoulAbilitySystemLibrary.GetLivePlayerWithRadius` _returnvalue (`|MakeArray` _returnvalue) 45.0 _returnvalue_4))
          (for _array_element _outoverlappingactors
            (`self.CauseDamage` _array_element))
          (`self.K2_EndAbility`))))
    (:`OnCompleted`
      (`self.K2_EndAbility` :!label _label))
    (:`OnInterrupted`
      (goto _label))
    (:`OnCancelled`
      (goto _label))))