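; Fire Bolt gameplay ability that casts a projectile toward a targeted location.
; A TargetData task supplies the hit location, and the avatar turns to face it through CombatInterface before playing the cast montage.
; The montage's Event.Montage.FireBolt gameplay event times the SpawnProjectile call, and the ability ends after a short delay.
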(event `self.K2_ActivateAbility`
  (bind (_asynctaskproxy _datahandle) (`TargetData.CreateTargetData`)
    (:`ValidData`
      (set `self.ProjectileTargetLocation` (`.Location` (`GameplayStatics.BreakHitResult` (`AbilitySystemBlueprintLibrary.GetHitResultFromTargetData` _datahandle))))
      (bind _ascombat_interface (cast `CombatInterface` (`self.GetAvatarActorFromActorInfo`)))
      (`CombatInterface.UpdateFacingTarget` _ascombat_interface (`self.ProjectileTargetLocation`))
      (`AbilityTask_PlayMontageAndWait.CreatePlayMontageAndWaitProxy` "None" "/Game/FabContent/ControlRig/Characters/Mannequins/Animations/StaffAnimation/AM_Cast_FireBolt.AM_Cast_FireBolt"
        (:`then`
          (`AbilityTask_WaitGameplayEvent.WaitGameplayEvent` (struct :`TagName` "Event.Montage.FireBolt") null
            (:`EventReceived`
              (`self.SpawnProjectile` (`self.ProjectileTargetLocation`))
              (`KismetSystemLibrary.Delay` 0.2)
              (`self.K2_EndAbility`))))))))