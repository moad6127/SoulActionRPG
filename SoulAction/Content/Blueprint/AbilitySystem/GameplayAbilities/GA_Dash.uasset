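; GA_Dash is a gameplay ability that performs a dash by playing a roll montage in the character's movement direction.
; On activation it rotates the avatar toward the direction from CombatInterface, saves and disables OrientRotationToMovement and controller-yaw rotation, then starts the montage.
; An Event.Montage.Dash gameplay event ends the ability, and OnEndAbility restores both saved rotation settings.
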(event `self.K2_ActivateAbility`
  (bind _ascombat_interface (cast `CombatInterface` (`self.GetAvatarActorFromActorInfo`)))
  (bind _returnvalue (`CombatInterface.GetMovementDirection` _ascombat_interface))
  (`Actor.K2_SetActorRotation` (`self.GetAvatarActorFromActorInfo`) (`KismetMathLibrary.Conv_VectorToRotator` _returnvalue) false)
  (bind `_as캐릭터` (cast `Character` (`self.GetAvatarActorFromActorInfo`)))
  (bind _output_get (set `self.Character` `_as캐릭터`))
  (bind _charactermovement (`Character.CharacterMovement` _output_get))
  (set `self.Orient Rotation To Movement` (`CharacterMovementComponent.bOrientRotationToMovement` _charactermovement))
  (set `CharacterMovementComponent.bOrientRotationToMovement` false _charactermovement)
  (set `self.Use Controller Rotation Yaw` (`Pawn.bUseControllerRotationYaw` (`self.Character`)))
  (set `Pawn.bUseControllerRotationYaw` false (`self.Character`))
  (`AbilityTask_PlayMontageAndWait.CreatePlayMontageAndWaitProxy` "None" "/Game/FabContent/ControlRig/Characters/Mannequins/Animations/AM_A_Roll.AM_A_Roll"
    (:`then`
      (`AbilityTask_WaitGameplayEvent.WaitGameplayEvent` (struct :`TagName` "Event.Montage.Dash") null
        (:`EventReceived`
          (`self.K2_EndAbility`))))))

(event `self.K2_OnEndAbility`
  (params (bWasCancelled :type Boolean))
  (bind `_as캐릭터` (cast `Character` (`self.GetAvatarActorFromActorInfo`)))
  (set `CharacterMovementComponent.bOrientRotationToMovement` (`self.Orient Rotation To Movement`) (`Character.CharacterMovement` `_as캐릭터`))
  (set `Pawn.bUseControllerRotationYaw` (`self.Use Controller Rotation Yaw`) (`self.Character`)))