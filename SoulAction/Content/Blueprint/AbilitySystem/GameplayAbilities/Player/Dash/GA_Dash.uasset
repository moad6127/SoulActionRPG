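; GA_Dash is a player gameplay ability that performs a short, fast dash in the character's movement direction.
; On activation it commits, then applies a constant-force root motion task along the direction from the avatar's CombatInterface.
; The dash gameplay cue is added until the ability ends, which happens when the task finishes.
; Exit velocity is clamped to BP_SoulCharacter's max movement speed, or zero for other avatars.
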(event `self.K2_ActivateAbility`
  (`self.K2_CommitAbility`)
  (`AbilityTask_ApplyRootMotionConstantForce.ApplyRootMotionConstantForce` "None" (`self.GetDashDirection`) 3000.0 0.3 false null "ClampVelocity" (0.0 0.0 0.0) (`self.GetMaxSpeed`)
    (:`then`
      (`self.K2_AddGameplayCue` (struct :`TagName` "GameplayCue.Dash")))
    (:`OnFinish`
      (`self.K2_EndAbility`))))

(fn `GetDashDirection`
  (returns (Direction :type "Vector Structure"))
  (bind _ascombat_interface (cast `CombatInterface` (`self.GetAvatarActorFromActorInfo`)))
  (bind _returnvalue (`CombatInterface.GetMovementDirection` _ascombat_interface))
  (return _returnvalue))

(fn `GetMaxSpeed`
  (returns (MaxSpeed :type "Float (double-precision)"))
  (bind _asbp_soul_character (cast `/Game/Blueprint/Character/BP_SoulCharacter` (`self.GetAvatarActorFromActorInfo`))
    (:`then`
      (return (`MovementComponent.GetMaxSpeed` (`Pawn.GetMovementComponent` _asbp_soul_character))))
    (:`CastFailed`
      (return 0.0))))