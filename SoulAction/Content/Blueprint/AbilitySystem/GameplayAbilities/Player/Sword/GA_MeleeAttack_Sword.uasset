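; Player sword melee attack gameplay ability that plays an attack montage and deals damage to actors the equipped weapon hits.
; Gameplay events for hit-scan start and end open and close the weapon's hit window, binding and unbinding its hit delegate.
; Each hit applies damage and fires a player melee impact gameplay cue at the weapon combat socket location.
; The ability ends when the montage completes, is interrupted or is cancelled.
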(event `self.K2_ActivateAbility`
  (bind _returnvalue (message `CombatInterface.GetEquippedWeapon` (`self.GetAvatarActorFromActorInfo`)))
  (set `self.EquippedWeapon` _returnvalue)
  (`AbilityTask_PlayMontageAndWait.CreatePlayMontageAndWaitProxy` "None" (`self.MeleeAttackMontage`) 1.0 "None" true 1.0 0.0 true
    (:`then`
      (`AbilityTask_WaitGameplayEvent.WaitGameplayEvent` (struct :`TagName` "Event.HitScan.Start") null
        (:`then`
          (`AbilityTask_WaitGameplayEvent.WaitGameplayEvent` (struct :`TagName` "Event.HitScan.End") null
            (:`EventReceived`
              (`BaseWeapon.HitScanEnd` (`self.EquippedWeapon`))
              (clear `BaseWeapon.OnWeaponHit` (`self.EquippedWeapon`)))))
        (:`EventReceived`
          (add `BaseWeapon.OnWeaponHit` (`self.EquippedWeapon`) (delegate `OnWeaponHit_이벤트`))
          (`BaseWeapon.HitScanStart` (`self.EquippedWeapon`)))))
    (:`OnCompleted`
      (`self.K2_EndAbility` :!label _label))
    (:`OnInterrupted`
      (goto _label))
    (:`OnCancelled`
      (goto _label))))

(event `OnWeaponHit_이벤트`
  (params (HitActor :type "Actor Object Reference"))
  (`self.CauseDamage` HitActor)
  (bind _returnvalue (message `CombatInterface.GetCombatSocketLocation` (`self.GetAvatarActorFromActorInfo`) (`BlueprintGameplayTagLibrary.MakeLiteralGameplayTag` (struct :`TagName` "CombatSocket.Weapon"))))
  (set `self.CombatLocation` _returnvalue)
  (`self.K2_ExecuteGameplayCueWithParams` (struct :`TagName` "GameplayCue.MeleeImpact.Player") (`AbilitySystemBlueprintLibrary.MakeGameplayCueParameters` 0.0 0.0 (struct) (struct) (struct) (struct) (struct) (`self.CombatLocation`) (0.0 0.0 0.0) null null (`self.GetAvatarActorFromActorInfo`))))